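; TextTimer is a level Blueprint actor that shows elapsed time on a TextRender component.
; A looping one-second timer started on BeginPlay calls Update, which increments a counter and rebuilds the "Time:" label.
; The label pairs the counter divided by 60 with the raw counter, both formatted to two digits, so the seconds field has no modulo 60.
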(event EventBeginPlay
  (Utilities|Time|SetTimerbyFunctionName 0 "Update" 1.0 true))

(fn ConstructionScript)

(fn Update
  ;[1 1 1] Increment counter
  (Variables|Default|SetTimesUpdated (+ (Variables|Default|GetTimesUpdated) 1))
  ;[1 1 1] Render
  (Rendering|Components|TextRender|SetText (Variables|Default|GetTextRender) (Utilities|String|Append "Time:" (Utilities|String|Append (Utilities|String|Append (Utilities|String|ToString(Text) (Utilities|Text|ToText(Integer) (/ (Variables|Default|GetTimesUpdated) 60) "HalfToEven" true 2 2)) ":") (Utilities|String|ToString(Text) (Utilities|Text|ToText(Integer) (Variables|Default|GetTimesUpdated) "HalfToEven" true 2 2))))))