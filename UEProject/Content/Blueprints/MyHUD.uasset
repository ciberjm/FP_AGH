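; HUD Blueprint that draws a centered crosshair and the player's bullet count on the canvas.
; DrawHUD passes the screen size to DrawCrosshair, which positions the texture by half its native size but draws it at a fixed 16x16.
; It then casts the player character to Player and prints BulletCount in red just below and right of the crosshair.
; DrawStats is an empty, uncalled stub.
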(event EventDrawHUD
  (params (SizeX :type Integer) (SizeY :type Integer))
  (CallFunction|DrawCrosshair SizeX SizeY))

(fn ConstructionScript)

(fn DrawCrosshair
  (params (ScreenSizeX :type Integer) (ScreenSizeY :type Integer))
  (bind _returnvalue (/ ScreenSizeY 2))
  (bind _returnvalue_2 (/ ScreenSizeX 2))
  (bind _crosshairtexture (Variables|Default|GetCrosshairTexture))
  (bind _returnvalue_3 (Class|Texture2D|BlueprintGetSizeX _crosshairtexture))
  (bind _returnvalue_4 (Class|Texture2D|BlueprintGetSizeY _crosshairtexture))
  (bind _returnvalue_5 (/ _returnvalue_4 2))
  (bind _returnvalue_6 (/ _returnvalue_3 2))
  (bind _returnvalue_7 (- _returnvalue _returnvalue_5))
  (bind _returnvalue_8 (- _returnvalue_2 _returnvalue_6))
  (bind _returnvalue_9 (Math|Conversions|ToFloat(Integer) _returnvalue_8))
  (bind _returnvalue_10 (Math|Conversions|ToFloat(Integer) _returnvalue_7))
  ;[1 1 1] Crosshair
  (Canvas|DrawTexture _crosshairtexture _returnvalue_9 _returnvalue_10 16.0 16.0 0.0 0.0 1.0 1.0 (Utilities|Struct|MakeLinearColor 1.0 1.0 1.0 1.0) "BLEND_Translucent" 1.0 true)
  (bind _asplayer_c (Utilities|Casting|CastToPlayer (Game|GetPlayerCharacter 0)))
  (HUD|DrawText (Utilities|String|BuildString(Integer) "" "" (Variables|/Game/Blueprints/Player/Player.Player_C|GetBulletCount _asplayer_c)) "(R=1.000000,G=0.000000,B=0.007827,A=1.000000)" (+ _returnvalue_9 18.0) (+ _returnvalue_10 18.0) 0 1.0 false))

(fn DrawStats
  (params (ScreenSizeX :type Integer) (ScreenSizeY :type Integer)))